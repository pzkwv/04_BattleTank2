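; Player-controllable tank Blueprint that maps input to movement, camera aiming and firing.
; BeginPlay hands turret and barrel references to setters and initialises TankMovement with both track components.
; Forward and turn axes feed TankMovement intents, aim axes rotate the azimuth gimbal and spring arm scaled by delta time, and the Fire action calls Fire.
; Per-track throttle axes ignore their input value and always set zero throttle.
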(event `self.ReceiveBeginPlay`
  (`self.SetTurretReference` (`self.TankTurret`))
  (`self.SetBarrelReference` (`self.Barrel`))
  (`TankMovementComponent.Initialise` (`self.TankMovement`) (`self.LeftTrackC`) (`self.RightTrackC`)))

(event `InputAxis|Left Track Throttle`
  (params (AxisValue :type "Float (single-precision)"))
  ;[1 1 1] Movement Input Binding
  (`TankTrack.SetThrottle` (`self.LeftTrackC`) 0.0))

(event `InputAxis|AimAzimuth`
  (params (AxisValue :type "Float (single-precision)"))
  ;[1 1 1] input setting
  (`SceneComponent.K2_AddLocalRotation` (`self.Azimuth Gimball`) (`KismetMathLibrary.MakeRotator` 0.0 0.0 (* AxisValue (`GameplayStatics.GetWorldDeltaSeconds`) 300.0)) false false))

(event `InputAxis|Right Track Throttle`
  (params (AxisValue :type "Float (single-precision)"))
  ;[1 1 1] Movement Input Binding
  (`TankTrack.SetThrottle` (`self.RightTrackC`) 0.0))

(event `InputAxis|AimElevation`
  (params (AxisValue :type "Float (single-precision)"))
  ;[1 1 1] input setting
  (`SceneComponent.K2_AddLocalRotation` (`self.SpringArm`) (`KismetMathLibrary.MakeRotator` 0.0 (* AxisValue (`GameplayStatics.GetWorldDeltaSeconds`) 300.0)) false false))

(event `InputAxis|ForBackward`
  (params (AxisValue :type "Float (single-precision)"))
  ;[1 1 1] Movement Input Binding
  (`TankMovementComponent.IntendMoveForward` (`self.TankMovement`) AxisValue))

(event `InputAxis|Turn Right`
  (params (AxisValue :type "Float (single-precision)"))
  ;[1 1 1] Movement Input Binding
  (`TankMovementComponent.IntendTurnRight` (`self.TankMovement`) AxisValue))

(event `InputAction|Fire`
  (params (Key :type "Key Structure"))
  ;[1 1 1] input setting
  (:`Pressed`
    (`self.Fire`)))

(fn `UserConstructionScript`)